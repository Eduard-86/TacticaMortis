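; Lobby HUD that shows each player's name, team and ready state in the slots of the main lobby widget.
; UpdateUI refreshes the widget, waits three ticks, then UpdateUILobby fills up to four slots from the game state's PlayerLobbyInfos.
; Only the authority or the name-matched owning player gets a slot enabled.
; Name, team and ready input handlers are empty, and their binding code is unreachable.
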(event `NameChange`
  (params (Text :type "Text (by ref)") (CommitMethod :type "ETextCommit Enum" :default "Default"))
  ;[0 0.15 0.115 0.5] УБЕРИ ДЕРЬМО
)

(event `ComandChange`
  (params (SelectedItem :type String) (SelectionType :type "ESelectInfo Enum" :default "OnKeyPress"))
  ;[0 0.15 0.115 0.5] УБЕРИ ДЕРЬМО
)

(event `CheckChanged`
  (params (bIsChecked :type Boolean))
  ;[0 0.15 0.115 0.5] УБЕРИ ДЕРЬМО
)

(event `self.ReceiveBeginPlay`
  (`parent.ReceiveBeginPlay`))

(event `self.UpdateUI`
  (`KismetSystemLibrary.PrintString` "Hello")
  (bind _aswbp_main_lobby_widget (cast `/Game/TacticaMortisContent/LevelSettings/Lobby/Widgets/MainLobbyWidget/WBP_MainLobbyWidget` (`self.MainWidget`)))
  (`KismetSystemLibrary.PrintString` "Hello")
  (`/Game/TacticaMortisContent/LevelSettings/Lobby/Widgets/MainLobbyWidget/WBP_MainLobbyWidget.UpdateInfo` _aswbp_main_lobby_widget)
  (`KismetSystemLibrary.DelayUntilNextTick`)
  (`KismetSystemLibrary.DelayUntilNextTick`)
  (`KismetSystemLibrary.DelayUntilNextTick`)
  (`self.UpdateUILobby`))

(fn `FindClientIndex`
  (params (LPC :type "LobbyPlayerController Object Reference"))
  (returns (PCIndex :type Integer))
  (bind _asbp_lobby_game_state (cast `/Game/TacticaMortisContent/LevelSettings/Lobby/BP_LobbyGameState` (`GameplayStatics.GetGameState`) :!pure true))
  (`/Engine/EditorBlueprintResources/StandardMacros.IsValid` _asbp_lobby_game_state
    (:`Is Valid`
      (for (_array_element _array_index) (`LobbyGameState.PlayerLobbyInfos` _asbp_lobby_game_state)
        (if (`KismetStringLibrary.EqualEqual_StrStr` (`.PlayerName` (break `PlayerLobbyInfo` _array_element)) (`PlayerState.GetPlayerName` (`Controller.PlayerState` LPC)))
          (return _array_index)))
      (return -1))
    (:`Is Not Valid`
      (return -1))))

(fn `UpdateUILobby`
  (bind _playerowner (`self.PlayerOwner`))
  (bind (_aswbp_main_lobby_widget _bsuccess) (cast `/Game/TacticaMortisContent/LevelSettings/Lobby/Widgets/MainLobbyWidget/WBP_MainLobbyWidget` (`self.MainWidget`) :!pure true))
  (bind _asbp_lobby_game_state (cast `/Game/TacticaMortisContent/LevelSettings/Lobby/BP_LobbyGameState` (`GameplayStatics.GetGameState`)))
  (if _bsuccess
    (for (_array_element _array_index) (`LobbyGameState.PlayerLobbyInfos` _asbp_lobby_game_state)
      (bind _returnvalue (select `int` _array_index :`0` (`/Game/TacticaMortisContent/LevelSettings/Lobby/Widgets/MainLobbyWidget/WBP_MainLobbyWidget.WBP_PlayerWidget1_0` _aswbp_main_lobby_widget) :`1` (`/Game/TacticaMortisContent/LevelSettings/Lobby/Widgets/MainLobbyWidget/WBP_MainLobbyWidget.WBP_PlayerWidget1_1` _aswbp_main_lobby_widget) :`2` (`/Game/TacticaMortisContent/LevelSettings/Lobby/Widgets/MainLobbyWidget/WBP_MainLobbyWidget.WBP_PlayerWidget1_2` _aswbp_main_lobby_widget) :`3` (`/Game/TacticaMortisContent/LevelSettings/Lobby/Widgets/MainLobbyWidget/WBP_MainLobbyWidget.WBP_PlayerWidget1_3` _aswbp_main_lobby_widget)))
      (`WidgetSwitcher.SetActiveWidgetIndex` (`/Game/TacticaMortisContent/LevelSettings/Lobby/Widgets/MainLobbyWidget/WBP_PlayerCard.WidgetSwitcher` _returnvalue) 0)
      (bind (_playeruniqueid _playername _teamindex _bisready) (break `PlayerLobbyInfo` _array_element))
      (`/Game/TacticaMortisContent/LevelSettings/Lobby/Widgets/MainLobbyWidget/WBP_PlayerCard.MakeEnableWidget` _returnvalue (or (`self.HasAuthority` _playerowner) (`KismetStringLibrary.EqualEqual_StrStr` (`PlayerState.GetPlayerName` (`Controller.PlayerState` _playerowner)) _playername)))
      (`EditableText.SetText` (`/Game/TacticaMortisContent/LevelSettings/Lobby/Widgets/MainLobbyWidget/WBP_PlayerCard.PlayerNameEditableTextBox` _returnvalue) (`KismetTextLibrary.Conv_StringToText` _playername))
      (`ComboBoxString.SetSelectedIndex` (`/Game/TacticaMortisContent/LevelSettings/Lobby/Widgets/MainLobbyWidget/WBP_PlayerCard.CommandComboBox` _returnvalue) _teamindex)
      (`CheckBox.SetCheckedState` (`/Game/TacticaMortisContent/LevelSettings/Lobby/Widgets/MainLobbyWidget/WBP_PlayerCard.ReadyCheckBox` _returnvalue) (select `bool` _bisready :`false` "Unchecked" :`true` "Checked" :!type "ECheckBoxState Enum")))))

(fn `UserConstructionScript`)