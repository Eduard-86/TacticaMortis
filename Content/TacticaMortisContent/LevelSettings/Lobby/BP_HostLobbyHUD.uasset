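; Lobby HUD that connects the main lobby widget to per-player lobby data for name, team and ready state.
; On BeginPlay it binds the widget's edit events to update calls keyed by slot index.
; UpdateUI waits three ticks, then fills the four player slots from the game state's PlayerLobbyInfos.
; Slots are editable with authority or when the local player's name matches, so identity relies on names.
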(event `CustomEvent`
  (params (WidgetIndex :type Integer) (NewName :type Text))
  (`self.UpdateWidgetPlayerNameByIndex` WidgetIndex (`KismetTextLibrary.Conv_TextToString` NewName)))

(event `CustomEvent_0`
  (params (WidgetIndex :type Integer) (TeamIndex :type Integer))
  (`self.UpdateWidgetPlayerTeamIndexByIndex` WidgetIndex TeamIndex))

(event `CustomEvent_1`
  (params (WidgetIndex :type Integer) (NewCheckState :type Boolean))
  (`self.UpdateWidgetPlayerReadyFlagByIndex` WidgetIndex NewCheckState))

(event `self.ReceiveBeginPlay`
  (`parent.ReceiveBeginPlay`)
  (`KismetSystemLibrary.PrintString` "Hello")
  (bind _aswbp_main_lobby_widget (cast `/Game/TacticaMortisContent/LevelSettings/Lobby/Widgets/MainLobbyWidget/WBP_MainLobbyWidget` (`self.MainWidget`)))
  (add `/Game/TacticaMortisContent/LevelSettings/Lobby/Widgets/MainLobbyWidget/WBP_MainLobbyWidget.PlayerNameEditableByWidgetIndex` _aswbp_main_lobby_widget (delegate `CustomEvent`))
  (add `/Game/TacticaMortisContent/LevelSettings/Lobby/Widgets/MainLobbyWidget/WBP_MainLobbyWidget.TeamChangeByWidgetIndex` _aswbp_main_lobby_widget (delegate `CustomEvent_0`))
  (add `/Game/TacticaMortisContent/LevelSettings/Lobby/Widgets/MainLobbyWidget/WBP_MainLobbyWidget.ReadyCheckChangeWidgetIndex` _aswbp_main_lobby_widget (delegate `CustomEvent_1`)))

(event `self.UpdateUI`
  (`KismetSystemLibrary.PrintString` "Hello")
  (`KismetSystemLibrary.DelayUntilNextTick`)
  (`KismetSystemLibrary.DelayUntilNextTick`)
  (`KismetSystemLibrary.DelayUntilNextTick`)
  (`self.UpdateUILobby`))

(fn `UpdateUILobby`
  (bind _playerowner (`self.PlayerOwner`))
  (bind (_aswbp_main_lobby_widget _bsuccess) (cast `/Game/TacticaMortisContent/LevelSettings/Lobby/Widgets/MainLobbyWidget/WBP_MainLobbyWidget` (`self.MainWidget`) :!pure true))
  (bind _asbp_lobby_game_state (cast `/Game/TacticaMortisContent/LevelSettings/Lobby/BP_LobbyGameState` (`GameplayStatics.GetGameState`)))
  (if _bsuccess
    (for (_array_element _array_index) (`LobbyGameState.PlayerLobbyInfos` _asbp_lobby_game_state)
      (bind _returnvalue (select `int` _array_index :`0` (`/Game/TacticaMortisContent/LevelSettings/Lobby/Widgets/MainLobbyWidget/WBP_MainLobbyWidget.WBP_PlayerWidget1_0` _aswbp_main_lobby_widget) :`1` (`/Game/TacticaMortisContent/LevelSettings/Lobby/Widgets/MainLobbyWidget/WBP_MainLobbyWidget.WBP_PlayerWidget1_1` _aswbp_main_lobby_widget) :`2` (`/Game/TacticaMortisContent/LevelSettings/Lobby/Widgets/MainLobbyWidget/WBP_MainLobbyWidget.WBP_PlayerWidget1_2` _aswbp_main_lobby_widget) :`3` (`/Game/TacticaMortisContent/LevelSettings/Lobby/Widgets/MainLobbyWidget/WBP_MainLobbyWidget.WBP_PlayerWidget1_3` _aswbp_main_lobby_widget)))
      (`WidgetSwitcher.SetActiveWidgetIndex` (`/Game/TacticaMortisContent/LevelSettings/Lobby/Widgets/MainLobbyWidget/WBP_PlayerCart.WidgetSwitcher` _returnvalue) 0)
      (bind (_playeruniqueid _playername _teamindex _bisready) (break `PlayerLobbyInfo` _array_element))
      (`/Game/TacticaMortisContent/LevelSettings/Lobby/Widgets/MainLobbyWidget/WBP_PlayerCart.MakeEnableWidget` _returnvalue (or (`self.HasAuthority` _playerowner) (`KismetStringLibrary.EqualEqual_StrStr` (`PlayerState.GetPlayerName` (`Controller.PlayerState` _playerowner)) _playername)))
      (`EditableText.SetText` (`/Game/TacticaMortisContent/LevelSettings/Lobby/Widgets/MainLobbyWidget/WBP_PlayerCart.PlayerNameEditableTextBox` _returnvalue) (`KismetTextLibrary.Conv_StringToText` _playername))
      (`ComboBoxString.SetSelectedIndex` (`/Game/TacticaMortisContent/LevelSettings/Lobby/Widgets/MainLobbyWidget/WBP_PlayerCart.CommandComboBox` _returnvalue) _teamindex)
      (`CheckBox.SetCheckedState` (`/Game/TacticaMortisContent/LevelSettings/Lobby/Widgets/MainLobbyWidget/WBP_PlayerCart.ReadyCheckBox` _returnvalue) (select `bool` _bisready :`false` "Unchecked" :`true` "Checked" :!type "ECheckBoxState Enum")))))

(fn `UserConstructionScript`
  (`parent.UserConstructionScript`))