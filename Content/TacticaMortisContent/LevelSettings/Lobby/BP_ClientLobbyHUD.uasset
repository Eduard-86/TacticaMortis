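; Client lobby HUD that links the main lobby widget to the local player's choices and the shared lobby game state.
; On BeginPlay it binds the local player's name, team and ready controls, plus character selection, to widget-update calls.
; UpdateUI refreshes the host card and three player cards from PlayerLobbyInfos, enabling cards only for their owner or authority, and locks map selection.
; Both binding and refresh first wait three ticks.
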(event `CustomEvent`
  (params (Text :type "Text (by ref)") (CommitMethod :type "ETextCommit Enum" :default "Default"))
  (`self.UpdateWidgetPlayerName` (`KismetTextLibrary.Conv_TextToString` Text)))

(event `CustomEvent_1`
  (params (SelectedItem :type String) (SelectionType :type "ESelectInfo Enum" :default "OnKeyPress"))
  (`self.UpdateWidgetPlayerTeamIndex` (`KismetStringLibrary.Conv_StringToInt` (`KismetStringLibrary.GetSubstring` SelectedItem 8))))

(event `CustomEvent_2`
  (params (bIsChecked :type Boolean))
  (`self.UpdateWidgetPlayerReadyFlag` bIsChecked))

(event `self.ReceiveBeginPlay`
  (bind _returnvalue (`LobbyGameState.FindPlayerInfoIndex` (cast `LobbyGameState` (`GameplayStatics.GetGameState`) :!pure true) (`self.PlayerOwner`)))
  (`parent.ReceiveBeginPlay`)
  (`KismetSystemLibrary.PrintString` "Hello")
  (`|ExecutionSequence`
    (:`then_0`
      (bind _aswbp_main_lobby_widget (cast `/Game/TacticaMortisContent/LevelSettings/Lobby/Widgets/MainLobbyWidget/WBP_MainLobbyWidget` (`self.MainWidget`)))
      ; Trahanii PlayerSatet
      (`KismetSystemLibrary.DelayUntilNextTick`)
      (`KismetSystemLibrary.DelayUntilNextTick`)
      (`KismetSystemLibrary.DelayUntilNextTick`)
      (bind _playerwidget (`/Game/TacticaMortisContent/LevelSettings/Lobby/Widgets/MainLobbyWidget/WBP_MainLobbyWidget.FindWidgetByIndex` _aswbp_main_lobby_widget _returnvalue))
      (if (!= _returnvalue -1)
        (add `EditableText.OnTextCommitted` (`/Game/TacticaMortisContent/LevelSettings/Lobby/Widgets/MainLobbyWidget/SubWudgets/WBP_PlayerCard.PlayerNameEditableTextBox` _playerwidget) (delegate `CustomEvent`))
        (add `ComboBoxString.OnSelectionChanged` (`/Game/TacticaMortisContent/LevelSettings/Lobby/Widgets/MainLobbyWidget/SubWudgets/WBP_PlayerCard.CommandComboBox` _playerwidget) (delegate `CustomEvent_1`))
        (add `CheckBox.OnCheckStateChanged` (`/Game/TacticaMortisContent/LevelSettings/Lobby/Widgets/MainLobbyWidget/SubWudgets/WBP_PlayerCard.ReadyCheckBox` _playerwidget) (delegate `CustomEvent_2`))))
    (:`then_1`
      (bind _aswbp_main_lobby_widget_2 (cast `/Game/TacticaMortisContent/LevelSettings/Lobby/Widgets/MainLobbyWidget/WBP_MainLobbyWidget` (`self.MainWidget`)))
      (add `/Game/TacticaMortisContent/LevelSettings/Lobby/Widgets/MainLobbyWidget/WBP_MainLobbyWidget.PlayerCharSelected` _aswbp_main_lobby_widget_2 (delegate `NewCharSelected`)))))

(event `NewCharSelected`
  (params (CharId :type Name))
  (`self.UpdateWidgetPlayerSelectCharacter` CharId))

(event `self.UpdateUI`
  (`KismetSystemLibrary.PrintString` "Hello")
  (`KismetSystemLibrary.DelayUntilNextTick`)
  (`KismetSystemLibrary.DelayUntilNextTick`)
  (`KismetSystemLibrary.DelayUntilNextTick`)
  (`self.UpdateUILobby`))

(fn `FindClientIndex`
  (params (LPC :type "LobbyPlayerController Object Reference"))
  (returns (PCIndex :type Integer))
  (bind _asbp_lobby_game_state (cast `/Game/TacticaMortisContent/LevelSettings/Lobby/BP_LobbyGameState` (`GameplayStatics.GetGameState`) :!pure true))
  (`/Engine/EditorBlueprintResources/StandardMacros.IsValid` _asbp_lobby_game_state
    (:`Is Valid`
      (for (_array_element _array_index) (`LobbyGameState.PlayerLobbyInfos` _asbp_lobby_game_state)
        (if (`KismetStringLibrary.EqualEqual_StrStr` (`.PlayerName` (break `PlayerLobbyInfo` _array_element)) (`PlayerState.GetPlayerName` (`Controller.PlayerState` LPC)))
          (return _array_index)))
      (return -1))
    (:`Is Not Valid`
      (return -1))))

(fn `UpdateUILobby`
  (bind _playerowner (`self.PlayerOwner`))
  (bind _aswbp_main_lobby_widget (cast `/Game/TacticaMortisContent/LevelSettings/Lobby/Widgets/MainLobbyWidget/WBP_MainLobbyWidget` (`self.MainWidget`) :!pure true))
  (bind (_aswbp_main_lobby_widget_2 _bsuccess) (cast `/Game/TacticaMortisContent/LevelSettings/Lobby/Widgets/MainLobbyWidget/WBP_MainLobbyWidget` (`self.MainWidget`) :!pure true))
  (bind _map_combobox (`/Game/TacticaMortisContent/LevelSettings/Lobby/Widgets/MainLobbyWidget/WBP_MainLobbyWidget.Map_ComboBox` _aswbp_main_lobby_widget))
  (bind _wbp_hostcard (`/Game/TacticaMortisContent/LevelSettings/Lobby/Widgets/MainLobbyWidget/WBP_MainLobbyWidget.WBP_HostCard` (cast `/Game/TacticaMortisContent/LevelSettings/Lobby/Widgets/MainLobbyWidget/WBP_MainLobbyWidget` (`self.MainWidget`) :!pure true)))
  (bind _asbp_lobby_game_state (cast `/Game/TacticaMortisContent/LevelSettings/Lobby/BP_LobbyGameState` (`GameplayStatics.GetGameState`)))
  (if _bsuccess
    (for (_array_element _array_index) (`LobbyGameState.PlayerLobbyInfos` _asbp_lobby_game_state)
      (if (== _array_index 0)
        (bind (_playeruniqueid _playername _teamindex _bisready _playercharacterrowname _assignedcharacterrownamesfromhost) (break `PlayerLobbyInfo` _array_element))
        (`/Game/TacticaMortisContent/LevelSettings/Lobby/Widgets/MainLobbyWidget/SubWudgets/WBP_HostCard.UpdateCharacterList` _wbp_hostcard _assignedcharacterrownamesfromhost)
        (`/Game/TacticaMortisContent/LevelSettings/Lobby/Widgets/MainLobbyWidget/SubWudgets/WBP_HostCard.MakeEnableWidget` _wbp_hostcard false)
        (else
          (bind _returnvalue (select `int` _array_index :`0` null :`1` (`/Game/TacticaMortisContent/LevelSettings/Lobby/Widgets/MainLobbyWidget/WBP_MainLobbyWidget.WBP_PlayerWidget1_1` _aswbp_main_lobby_widget_2) :`2` (`/Game/TacticaMortisContent/LevelSettings/Lobby/Widgets/MainLobbyWidget/WBP_MainLobbyWidget.WBP_PlayerWidget1_2` _aswbp_main_lobby_widget_2) :`3` (`/Game/TacticaMortisContent/LevelSettings/Lobby/Widgets/MainLobbyWidget/WBP_MainLobbyWidget.WBP_PlayerWidget1_3` _aswbp_main_lobby_widget_2)))
          (`WidgetSwitcher.SetActiveWidgetIndex` (`/Game/TacticaMortisContent/LevelSettings/Lobby/Widgets/MainLobbyWidget/SubWudgets/WBP_PlayerCard.WidgetSwitcher` _returnvalue) 0)
          (`/Game/TacticaMortisContent/LevelSettings/Lobby/Widgets/MainLobbyWidget/SubWudgets/WBP_PlayerCard.MakeEnableWidget` _returnvalue (or (`self.HasAuthority` _playerowner) (`KismetStringLibrary.EqualEqual_StrStr` (`PlayerState.GetPlayerName` (`Controller.PlayerState` _playerowner)) _playername)))
          (`EditableText.SetText` (`/Game/TacticaMortisContent/LevelSettings/Lobby/Widgets/MainLobbyWidget/SubWudgets/WBP_PlayerCard.PlayerNameEditableTextBox` _returnvalue) (`KismetTextLibrary.Conv_StringToText` _playername))
          (`ComboBoxString.SetSelectedIndex` (`/Game/TacticaMortisContent/LevelSettings/Lobby/Widgets/MainLobbyWidget/SubWudgets/WBP_PlayerCard.CommandComboBox` _returnvalue) _teamindex)
          (`CheckBox.SetCheckedState` (`/Game/TacticaMortisContent/LevelSettings/Lobby/Widgets/MainLobbyWidget/SubWudgets/WBP_PlayerCard.ReadyCheckBox` _returnvalue) (select `bool` _bisready :`false` "Unchecked" :`true` "Checked" :!type "ECheckBoxState Enum"))
          (`/Game/TacticaMortisContent/LevelSettings/Lobby/Widgets/MainLobbyWidget/SubWudgets/WBP_PlayerCard.SetCharSelected` _returnvalue _playercharacterrowname)
          (`/Game/TacticaMortisContent/LevelSettings/Lobby/Widgets/MainLobbyWidget/SubWudgets/WBP_PlayerCard.UpdateCharList` (cast `/Game/TacticaMortisContent/LevelSettings/Lobby/Widgets/MainLobbyWidget/SubWudgets/WBP_PlayerCard` (`PanelWidget.GetChildAt` (`/Game/TacticaMortisContent/LevelSettings/Lobby/Widgets/MainLobbyWidget/WBP_MainLobbyWidget.HostsScrollBox` _aswbp_main_lobby_widget) _array_index) :!pure true) _assignedcharacterrownamesfromhost)
          (`ComboBoxString.SetSelectedOption` _map_combobox (`KismetStringLibrary.Conv_NameToString` (`LobbyGameState.SelectMap` (cast `LobbyGameState` (`GameplayStatics.GetGameState`) :!pure true))))
          (`Widget.SetIsEnabled` _map_combobox false))))))

(fn `UserConstructionScript`
  (`parent.UserConstructionScript`))