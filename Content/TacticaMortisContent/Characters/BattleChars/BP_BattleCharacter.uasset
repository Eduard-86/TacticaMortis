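; Battle character that tints its skin by race and roams the navmesh at random.
; On BeginPlay it waits three ticks, then looks up its CharRowName row in DT_CharData.
; If the row is found, it applies a dynamic skin material colored by the Race attribute and starts a looping timer.
; Each timer tick sends its controller to a random navigable point via SimpleMoveToLocation.
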(event `self.ReceiveBeginPlay`
  (`KismetSystemLibrary.DelayUntilNextTick`)
  (`KismetSystemLibrary.DelayUntilNextTick`)
  (`KismetSystemLibrary.DelayUntilNextTick`)
  (bind _returnvalue (`|GetDataTableRow` "/Game/TacticaMortisContent/Characters/DT_CharData.DT_CharData" (`self.CharRowName`))
    (:`then`
      (bind _returnvalue_2 (`KismetMaterialLibrary.CreateDynamicMaterialInstance` "/Game/TacticaMortisContent/Assets/Materials/M_RaceSkine.M_RaceSkine"))
      (`MaterialInstanceDynamic.SetVectorParameterValue` _returnvalue_2 "ColorInput" (select `int` (`KismetMathLibrary.Conv_ByteToInt` (`.Race` (break `CharacterAttributes` (`.Attributes` (break `CharacterData` _returnvalue))))) :`0` (struct :`R` 0.034289 :`G` 0.002148 :`B` 1.0 :`A` 1.0) :`1` (struct :`R` 0.063183 :`G` 1.0 :`A` 1.0) :`2` (struct :`R` 1.0 :`G` 0.046009 :`A` 1.0) :!type "LinearColor Structure"))
      (`PrimitiveComponent.SetMaterial` (`self.Mesh`) 0 _returnvalue_2)
      (`KismetSystemLibrary.K2_SetTimerDelegate` (delegate `CustomEvent`) 2.0 true))))

(event `CustomEvent`
  (bind _randomlocation (`NavigationSystemV1.K2_GetRandomLocationInNavigableRadius` (0.0 0.0 0.0) 800.0 null null))
  (`AIBlueprintHelperLibrary.SimpleMoveToLocation` (`self.GetController`) _randomlocation))

(fn `UserConstructionScript`)